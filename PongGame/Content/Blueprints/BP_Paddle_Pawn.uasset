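; BP_Paddle_Pawn is a player paddle pawn, apparently for a Pong-style game, moved along the X axis by physics.
; Each tick it adds force to PaddleMesh scaled by the P1_moveup input axis.
; When the actor passes either X limit, it snaps just inside that bound instead of applying force, keeping the paddle within the play area.
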(event EventTick
  (params (DeltaSeconds :type Float%20%28single-precision%29))
  (bind _returnvalue (Transformation|GetActorLocation))
  (bind _returnvalue_2 (Transformation|GetActorLocation))
  (bind (_x _y _z) (Math|Vector|BreakVector _returnvalue))
  (bind (_x_2 _y_2 _z_2) (Math|Vector|BreakVector _returnvalue_2))
  (if (> (.X (Math|Vector|BreakVector (Transformation|GetActorLocation))) 4e+02)
    (Transformation|SetActorLocation (Math|Vector|MakeVector 399.899994 _y _z) false false)
    (elif (< (.X (Math|Vector|BreakVector (Transformation|GetActorLocation))) -4e+02)
      (Transformation|SetActorLocation (Math|Vector|MakeVector -399.899994 _y_2 _z_2) false false)
      (else
        (Physics|AddForce (Variables|Default|GetPaddleMesh) (Math|Vector|MakeVector (* (Input|AxisValues|GetP1_moveup) 1e+05) 0.0 0.0) "None" false)))))

(fn ConstructionScript)