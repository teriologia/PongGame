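; BP_Ball is the ball in a Pong-style game, launched along Y at BeginPlay and driven by setting physics linear velocity.
; On overlap, player and AI paddles reverse its Y and set X from paddle velocity plus random spread, while horizontal walls reverse X.
; Goals recenter and relaunch it, increment the opposite side's score stored on the ball, and update TextRenderActors found by root component tag.
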(event EventBeginPlay
  (Physics|SetPhysicsLinearVelocity (Variables|Default|GetStaticMesh) "0,500.000000, 0" false "None"))

(event Collision|EventActorBeginOverlap
  (params (OtherActor :type Actor%20Object%20Reference))
  (bind _staticmesh (Variables|Default|GetStaticMesh))
  (bind _asbp_paddle_pawn (Utilities|Casting|CastToBP_Paddle_Pawn OtherActor)
    (:then
      (bind _returnvalue (Physics|GetPhysicsLinearVelocity (Variables|/Game/Blueprints/BP_Paddle_Pawn.BP_Paddle_Pawn_C|GetPaddleMesh _asbp_paddle_pawn) "None"))
      (bind _returnvalue_2 (Physics|GetPhysicsLinearVelocity _staticmesh "None"))
      (Physics|SetPhysicsLinearVelocity _staticmesh (Math|Vector|MakeVector (+ (.X (Math|Vector|BreakVector _returnvalue)) (Math|Random|RandomFloatinRange -2e+02 2e+02)) (* (.Y (Math|Vector|BreakVector _returnvalue_2)) -1.0) (.Z (Math|Vector|BreakVector _returnvalue_2))) false "None"))
    (:CastFailed
      (bind _asbp_ai_paddle (Utilities|Casting|CastToBP_AI_Paddle OtherActor)
        (:then
          (bind _returnvalue_3 (Physics|GetPhysicsLinearVelocity (Variables|/Game/Blueprints/BP_AI_Paddle.BP_AI_Paddle_C|GetStaticMesh _asbp_ai_paddle) "None"))
          (bind _returnvalue_4 (Physics|GetPhysicsLinearVelocity _staticmesh "None"))
          (Physics|SetPhysicsLinearVelocity _staticmesh (Math|Vector|MakeVector (+ (.X (Math|Vector|BreakVector _returnvalue_3)) (Math|Random|RandomFloatinRange -2e+02 2e+02)) (* (.Y (Math|Vector|BreakVector _returnvalue_4)) -1.0) (.Z (Math|Vector|BreakVector _returnvalue_4))) false "None"))
        (:CastFailed
          (Utilities|Casting|CastToBP_HorizontalWall OtherActor
            (:then
              (bind _returnvalue_5 (Physics|GetPhysicsLinearVelocity _staticmesh "None"))
              (Physics|SetPhysicsLinearVelocity _staticmesh (Math|Vector|MakeVector (* (.X (Math|Vector|BreakVector _returnvalue_5)) -1.0) (.Y (Math|Vector|BreakVector _returnvalue_5)) (.Z (Math|Vector|BreakVector _returnvalue_5))) false "None"))
            (:CastFailed
              (Utilities|Casting|CastToBP_L_Goal OtherActor
                (:then
                  (Transformation|SetActorLocation "0, 0, 0" false false)
                  (Physics|SetPhysicsLinearVelocity (Variables|Default|GetStaticMesh) "0,500.000000, 0" false "None")
                  (Variables|Default|SetR_Player_scroe (+ (Variables|Default|GetR_Player_scroe) 1))
                  (bind _outactors (Actor|GetAllActorsOfClass "/Script/Engine.TextRenderActor"))
                  (for _array_element _outactors
                    (bind _astext_render_actor (Utilities|Casting|CastToTextRenderActor _array_element))
                    (if (Components|ComponentHasTag (Variables|/Script/Engine.Actor|GetRootComponent _astext_render_actor) "rightScore")
                      (Rendering|Components|TextRender|SetText (Variables|/Script/Engine.TextRenderActor|GetTextRender _astext_render_actor) (Utilities|Text|ToText(Integer) (Variables|Default|GetR_Player_scroe))))))
                (:CastFailed
                  (Utilities|Casting|CastToBP_R_Goal OtherActor)
                  (Transformation|SetActorLocation "0, 0, 0" false false)
                  (Physics|SetPhysicsLinearVelocity _staticmesh "0,-500.000000, 0" false "None")
                  (Variables|Default|SetL_Player_score (+ (Variables|Default|GetL_Player_score) 1))
                  (bind _outactors_2 (Actor|GetAllActorsOfClass "/Script/Engine.TextRenderActor"))
                  (for _array_element_2 _outactors_2
                    (bind _astext_render_actor_2 (Utilities|Casting|CastToTextRenderActor _array_element_2))
                    (if (Components|ComponentHasTag (Variables|/Script/Engine.Actor|GetRootComponent _astext_render_actor_2) "leftScore")
                      (Rendering|Components|TextRender|SetText (Variables|/Script/Engine.TextRenderActor|GetTextRender _astext_render_actor_2) (Utilities|Text|ToText(Integer) (Variables|Default|GetL_Player_score))))))))))))))

(event EventTick
  (params (DeltaSeconds :type Float%20%28single-precision%29)))

(fn ConstructionScript)